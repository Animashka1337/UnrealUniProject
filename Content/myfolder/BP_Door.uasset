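; BP_Door is a door actor that snaps between closed and open positions when its OpenDoor and CloseDoor events are called.
; BeginPlay caches Cube3's relative location as the closed position and adds OffsetValue to derive the open one.
; Each event moves the cube instantly and toggles two spheres as state indicators, one visible while closed and the other while open.
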(event Custom|CloseDoor
  (Transformation|SetRelativeLocation (Variables|Default|GetCube3) (Variables|Default|GetClosedLocation) false false)
  (Rendering|SetVisibility (Variables|Default|GetSphere) true false)
  (Rendering|SetVisibility (Variables|Default|GetSphere1) false false))

(event Custom|OpenDoor
  (Transformation|SetRelativeLocation (Variables|Default|GetCube3) (Variables|Default|GetOpenLocation) false false)
  (Rendering|SetVisibility (Variables|Default|GetSphere) false false)
  (Rendering|SetVisibility (Variables|Default|GetSphere1) true false))

(event EventBeginPlay
  (bind _output_get (Variables|Default|SetClosedLocation (Variables|/Script/Engine.SceneComponent|GetRelativeLocation (Variables|Default|GetCube3))))
  (Variables|Default|SetOpenLocation (+ _output_get (Variables|Default|GetOffsetValue)))
  (Rendering|SetVisibility (Variables|Default|GetSphere) true false)
  (Rendering|SetVisibility (Variables|Default|GetSphere1) false false))

(event Collision|EventActorBeginOverlap
  (params (OtherActor :type Actor%20Object%20Reference)))

(event EventTick
  (params (DeltaSeconds :type Float%20%28single-precision%29)))

(fn ConstructionScript)