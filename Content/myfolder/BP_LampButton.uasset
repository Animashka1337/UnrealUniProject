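; BP_LampButton is an interactable button that lights a set of lamps when the player triggers it.
; A Box overlap with BP_Michelle stores that character as PlayerNearby and enables input, while leaving disables input without clearing the reference.
; IA_Interact calls SetLit on every entry in Lamps, provided PlayerNearby is valid and IsLocked is false.
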(event OnComponentBeginOverlap(Box)
  (params (OverlappedComponent :type Primitive%20Component%20Object%20Reference) (OtherActor :type Actor%20Object%20Reference) (OtherComp :type Primitive%20Component%20Object%20Reference) (OtherBodyIndex :type Integer) (bFromSweep :type Boolean) (SweepResult :type Hit%20Result%20Structure%20%28by%20ref%29))
  (bind _asbp_michelle (Utilities|Casting|CastToBP_Michelle OtherActor))
  (Variables|Default|SetPlayerNearby _asbp_michelle)
  (Input|EnableInput (Game|GetPlayerController 0)))

(event OnComponentEndOverlap(Box)
  (params (OverlappedComponent :type Primitive%20Component%20Object%20Reference) (OtherActor :type Actor%20Object%20Reference) (OtherComp :type Primitive%20Component%20Object%20Reference) (OtherBodyIndex :type Integer))
  (bind _asbp_michelle (Utilities|Casting|CastToBP_Michelle OtherActor))
  (Variables|Default|SetPlayerNearby _asbp_michelle)
  (Input|DisableInput (Game|GetPlayerController 0)))

(event Input|EnhancedActionEvents|EnhancedInputActionIA_Interact
  (params (ActionValue :type Boolean) (ElapsedSeconds :type Float%20%28double-precision%29) (TriggeredSeconds :type Float%20%28double-precision%29) (InputAction :type Input%20Action%20Object%20Reference :default "/Game/Input/Actions/IA_Interact.IA_Interact"))
  (:Started
    (Utilities|IsValid (Variables|Default|GetPlayerNearby)
      (:Is%20Valid
        (if (not (Variables|Default|GetIsLocked))
          (for _array_element (Variables|Default|GetLamps)
            (Default|SetLit _array_element)))))))

(fn ConstructionScript)