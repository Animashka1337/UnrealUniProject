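; BP_PuzzleLamp is a puzzle lamp actor that switches between lit and unlit states.
; SetLit acts as a toggle, flipping IsLit and showing the Sphere component when lit or hiding it when unlit.
; Each toggle broadcasts the OnLampChanged event dispatcher.
; BeginPlay resets IsLit to false without touching the Sphere's visibility.
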(event EventBeginPlay
  (Variables|Default|SetIsLit false))

(fn ConstructionScript)

(fn SetLit
  (bind _sphere (Variables|Default|GetSphere))
  (if (Variables|Default|GetIsLit)
    (Development|SetHiddeninGame _sphere true false)
    (Variables|Default|SetIsLit false)
    (Default|CallOnLampChanged)
    (else
      (Development|SetHiddeninGame _sphere false false)
      (Variables|Default|SetIsLit true)
      (Default|CallOnLampChanged))))