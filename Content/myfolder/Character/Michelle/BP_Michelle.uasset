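; Michelle player character Blueprint that handles Enhanced Input movement, mouse look, aiming, sprinting and crouching.
; Aiming is blocked while running and narrows camera FOV through a timeline, while sprint raises walk speed only when not aiming.
; Crouching slows movement and shrinks the capsule through a timeline.
; On crouch release, an upward sphere trace retries on a short delay until headroom is clear, then restores walk speed and capsule height.
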(event Custom|StandUP
  ;[0.15 0.15 0.15 0.5] Crouch Handling
  (Variables|/Script/Engine.CharacterMovementComponent|SetMaxWalkSpeed (Variables|Character|GetCharacterMovement) (Variables|Default|GetWalk))
  (bind _newtrack_0 (Timeline|Timeline Reverse)
    (:Update
      (CallFunction|UpdateCapsule _newtrack_0))))

(event Custom|CheckForObstruction
  (bind (_start _end) (CallFunction|GetSphereTraceEnd))
  ;[0.15 0.15 0.15 0.5] Crouch Handling
  (if (not (Variables|Default|GetIsCrouching)) :!label _label
    (bind _returnvalue (Collision|SphereTraceByChannel _start _end 0.0 "TraceTypeQuery1" false 0 "None"))
    (if _returnvalue
      (Utilities|FlowControl|Delay 0.2)
      (goto _label)
      (else
        (CallFunction|StandUP)))))

(event Input|EnhancedActionEvents|EnhancedInputActionIA_Aim
  (params (ActionValue :type Boolean) (ElapsedSeconds :type Float%20%28double-precision%29) (TriggeredSeconds :type Float%20%28double-precision%29) (InputAction :type Input%20Action%20Object%20Reference :default "/Game/myfolder/IA_Aim.IA_Aim"))
  ;[0.15 0.15 0.15 0.5] Aim Handling
  (:Started
    (if (not (Variables|Default|GetIsRunning))
      (Variables|Default|SetISAiming true)
      (bind _aboba (Timeline|Change%20FOV Play)
        (:Update
          (Camera|SetFieldOfView (Variables|Default|GetCamera) (Math|Float|Lerp 9e+01 7e+01 _aboba))))))
  (:Completed
    (if (Variables|Default|GetISAiming)
      (Variables|Default|SetISAiming false)
      (Timeline|Change%20FOV Reverse))))

(event Input|EnhancedActionEvents|EnhancedInputActionIA_MouseLook
  (params (ActionValue :type Vector%202D%20Structure) (ElapsedSeconds :type Float%20%28double-precision%29) (TriggeredSeconds :type Float%20%28double-precision%29) (InputAction :type Input%20Action%20Object%20Reference :default "/Game/Input/Actions/IA_MouseLook.IA_MouseLook"))
  ;[0.15 0.15 0.15 0.5] Movement and Camera handling
  (Pawn|Input|AddControllerYawInput (.x ActionValue))
  (Pawn|Input|AddControllerPitchInput (.y ActionValue)))

(event Input|EnhancedActionEvents|EnhancedInputActionIA_Move
  (params (ActionValue :type Vector%202D%20Structure) (ElapsedSeconds :type Float%20%28double-precision%29) (TriggeredSeconds :type Float%20%28double-precision%29) (InputAction :type Input%20Action%20Object%20Reference :default "/Game/Input/Actions/IA_Move.IA_Move"))
  (bind _returnvalue (Pawn|GetControlRotation :!class /Script/Engine.Pawn))
  ;[0.15 0.15 0.15 0.5] Movement and Camera handling
  (if (Variables|Default|GetCanMove)
    (Pawn|Input|AddMovementInput (Math|Vector|GetRightVector (Pawn|GetControlRotation :!class /Script/Engine.Pawn)) (.x ActionValue) false)
    (Pawn|Input|AddMovementInput (Math|Vector|GetForwardVector (Math|Rotator|MakeRotator (.roll _returnvalue) 0.0 (.yaw _returnvalue))) (.y ActionValue) false)))

(event Input|EnhancedActionEvents|EnhancedInputActionIA_Crouch
  (params (ActionValue :type Boolean) (ElapsedSeconds :type Float%20%28double-precision%29) (TriggeredSeconds :type Float%20%28double-precision%29) (InputAction :type Input%20Action%20Object%20Reference :default "/Game/myfolder/IA_Crouch.IA_Crouch"))
  ;[0.15 0.15 0.15 0.5] Crouch Handling
  (:Triggered
    (Variables|Default|SetIsCrouching true)
    (Variables|Default|SetIsRunning false)
    (Variables|/Script/Engine.CharacterMovementComponent|SetMaxWalkSpeed (Variables|Character|GetCharacterMovement) (Variables|Default|GetCrawlSpeed))
    (bind _newtrack_0 (Timeline|Timeline Play)
      (:Update
        (CallFunction|UpdateCapsule _newtrack_0))))
  (:Completed
    (Variables|Default|SetIsCrouching false)
    (CallFunction|CheckforObstruction)))

(event Input|EnhancedActionEvents|EnhancedInputActionIA_Sprint
  (params (ActionValue :type Boolean) (ElapsedSeconds :type Float%20%28double-precision%29) (TriggeredSeconds :type Float%20%28double-precision%29) (InputAction :type Input%20Action%20Object%20Reference :default "/Game/myfolder/IA_Sprint.IA_Sprint"))
  (bind _charactermovement (Variables|Character|GetCharacterMovement))
  ;[0.15 0.15 0.15 0.5] Sprint Handling
  (:Triggered
    (Variables|Default|SetIsRunning true :!label _label)
    (if (not (Variables|Default|GetISAiming))
      (Variables|/Script/Engine.CharacterMovementComponent|SetMaxWalkSpeed _charactermovement (Variables|Default|GetSprint))))
  (:Ongoing
    (goto _label))
  (:Completed
    (Variables|Default|SetIsRunning false)
    (Variables|/Script/Engine.CharacterMovementComponent|SetMaxWalkSpeed _charactermovement (Variables|Default|GetWalk))))

(event EventBeginPlay
  (bind _returnvalue (Game|GetPlayerController 0))
  (bind _returnvalue_2 (PlayerController|LocalPlayerSubsystems|GetEnhancedInputLocalPlayerSubsystem _returnvalue))
  ;[0.15 0.15 0.15 0.5] Input adding
  (Utilities|IsValid _returnvalue_2
    (:Is%20Valid
      (Input|AddMappingContext _returnvalue_2 "/Game/myfolder/IMC_Michelle.IMC_Michelle" 0 "(bIgnoreAllPressedKeysUntilRelease=True,bForceImmediately=False,bNotifyUserSettings=False)"))))

(event Input|KeyboardEvents|LeftShift
  (params (Key :type Key%20Structure :default "None"))
  ;[0.15 0.15 0.15 0.5] Sprint Handling
)

(fn ConstructionScript)

(fn UpdateCapsule
  (params (CrouchAlpha :type Float%20%28double-precision%29))
  (Components|Capsule|SetCapsuleHalfHeight (Variables|Collision|GetCapsuleComponent) (Math|Float|Lerp (Variables|Default|GetCapsuleHeight) (Variables|Default|GetCrawlCapsuleHeight) CrouchAlpha) true))

(fn GetSphereTraceEnd
  (bind _capsulecomponent (Variables|Collision|GetCapsuleComponent))
  (bind _returnvalue (Transformation|GetWorldLocation _capsulecomponent))
  (return (+ _returnvalue "0.000000,0.000000,30.000000") (+ _returnvalue "0.000000,0.000000,90.000000")))